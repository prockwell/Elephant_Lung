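; BP_Meteor is a falling meteor actor for the DinoGame that explodes when it overlaps another actor.
; Tick moves it down its local Z axis at Speed until IsDead is set.
; On overlap, Explode sets that flag, activates the PExplosion effect and destroys the Sphere component, leaving the actor in place.
; DoDamage only prints the hit actor's name, and a timed MoveComponentTo descent is left unconnected.
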(event `self.ReceiveBeginPlay`)

(event `self.ReceiveActorBeginOverlap`
  (params (OtherActor :type "Actor Object Reference"))
  (`self.Explode`)
  (`self.DoDamage` OtherActor))

(event `self.ReceiveTick`
  (params (DeltaSeconds :type "Float (single-precision)"))
  (if (not (`self.IsDead`))
    (`self.MoveDown` DeltaSeconds)))

(fn `DoDamage`
  (params (OtherActors :type "Actor Object Reference"))
  (`KismetSystemLibrary.PrintString` (`KismetStringLibrary.Concat_StrStr` "COLLISION: " (`KismetSystemLibrary.GetObjectName` OtherActors))))

(fn `Explode`
  (set `self.IsDead` true)
  (`ActorComponent.Activate` (`self.P_Explosion`) false)
  (`ActorComponent.K2_DestroyComponent` (`self.Sphere`)))

(fn `MoveDown`
  (params (DT :type "Float (double-precision)"))
  (`self.K2_AddActorLocalOffset` (`KismetMathLibrary.MakeVector` 0.0 0.0 (* DT (`self.Speed`) -1.0))))

(fn `UserConstructionScript`)