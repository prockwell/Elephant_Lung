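; BP_Egg is a one-time pickup that a BP_DinoCharacter eats by overlapping it.
; On overlap it calls Eat on the character, destroys its static mesh and activates the PSparks effect.
; An IsDead flag, set before the delays, blocks repeat triggers while the sparks briefly play, then the effect deactivates and the actor destroys itself.
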(event `self.ReceiveActorBeginOverlap`
  (params (OtherActor :type "Actor Object Reference"))
  (bind _p_sparks (`self.P_Sparks`))
  (if (not (`self.IsDead`))
    (bind _asbp_dino_character (cast `/Game/DinoGame/BP_DinoCharacter` OtherActor))
    (`/Game/DinoGame/BP_DinoCharacter.Eat` _asbp_dino_character)
    (`ActorComponent.K2_DestroyComponent` (`self.StaticMesh`))
    (`ActorComponent.Activate` _p_sparks false)
    (set `self.IsDead` true)
    (`KismetSystemLibrary.Delay` 0.2)
    (`ActorComponent.Deactivate` _p_sparks)
    (`KismetSystemLibrary.Delay` 1.0)
    (`self.K2_DestroyActor`)))

(fn `UserConstructionScript`)