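; Meteor spawner for the dino game that runs the "Ragnarok" phase, raining BP_Meteor actors at random points inside a box volume.
; The player controller's start-game event starts a timer, or a flag skips the wait, and StartRagnarok enables Tick and crossfades the music.
; Tick ramps a danger ratio to one, shortening spawn intervals and enlarging randomly scaled meteors, and prints debug values.
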(event `self.ReceiveBeginPlay`
  (bind _asbp_dino_controller (cast `/Game/DinoGame/BP_DinoController` (`GameplayStatics.GetPlayerController` 0)))
  ;[1 1 1] Start Game and Start Ragnarok Events
  (add `/Game/DinoGame/BP_DinoController.StartGameEvent` _asbp_dino_controller (delegate `OnStartGameEvent`))
  (bind _returnvalue (`GameplayStatics.SpawnSound2D` "/Game/DinoGame/Audio/Music/Pangea_Cue.Pangea_Cue" 1.0 1.0 0.0 null))
  (set `self.MusicSound` _returnvalue)
  (if (`self.StartWithRagnarok`)
    (`self.StartRagnarok`)))

(event `OnStartGameEvent`
  ;[1 1 1] Start Game and Start Ragnarok Events
  (`KismetSystemLibrary.K2_SetTimerDelegate` (delegate `OnStartRagnarokEvent`) (`self.TimeBeforeRagnarok`))
  (clear `/Game/DinoGame/BP_DinoController.StartGameEvent` (stale `self.ReceiveBeginPlay` _asbp_dino_controller)))

(event `OnStartRagnarokEvent`
  ;[1 1 1] Start Game and Start Ragnarok Events
  (`self.StartRagnarok`))

(event `self.ReceiveTick`
  (params (DeltaSeconds :type "Float (single-precision)"))
  (`|ExecutionSequence`
    (:`then_0`
      ;[1 1 1] Spawn Meteor
      (bind _output_get (set `self.SpawnTime` (- (`self.SpawnTime`) (* DeltaSeconds (`self.SpawnTimeSpeed`)))))
      (if (<= _output_get 0.0)
        (`self.SpawnMeteor`)
        (set `self.SpawnTime` (`KismetMathLibrary.FMax` (* (`self.MaxSpawnTime`) (- 1.0 (`self.RagnarokDangerRatio`))) (* (`KismetMathLibrary.RandomFloat`) 0.5)))))
    (:`then_1`
      (bind _output_get_2 (set `self.RagnarokDangerRatio` (`KismetMathLibrary.FClamp` (+ (`self.RagnarokDangerRatio`) (/ DeltaSeconds (`self.MaxDangerTime`))))))
      (`KismetSystemLibrary.PrintString` (`KismetStringLibrary.Concat_StrStr` "DANGER: " (`KismetStringLibrary.Conv_DoubleToString` _output_get_2)) true true (struct :`R` 1.0 :`G` 0.24044 :`B` 0.845292 :`A` 1.0) 2.0 "danger "))
    (:`then_2`
      (`KismetSystemLibrary.PrintString` (`KismetStringLibrary.Concat_StrStr` "SPAWN TIME: " (`KismetStringLibrary.Conv_DoubleToString` (`self.SpawnTime`))) true true (struct :`R` 0.181597 :`G` 0.174385 :`B` 1.0 :`A` 1.0) 2.0 "spawn"))
    (:`then_3`
      (bind _isragnarok (`self.GetIsRagnarok`))
      (`KismetSystemLibrary.PrintString` (`KismetStringLibrary.Concat_StrStr` "RAGNAROK: " (`KismetStringLibrary.Conv_BoolToString` _isragnarok)) true true (struct :`R` 1.0 :`G` 0.859266 :`B` 0.014152 :`A` 1.0) 2.0 "ragnarok"))))

(fn `GetIsRagnarok`
  (returns (IsRagnarok :type Boolean))
  (return (> (`self.TimeBeforeRagnarok`) 0.0)))

(fn `SpawnMeteor`
  (`|SpawnActorFromClass` "/Game/DinoGame/BP_Meteor.BP_Meteor_C" (`KismetMathLibrary.MakeTransform` (`KismetMathLibrary.RandomPointInBoundingBox` (.location (`SceneComponent.GetRelativeTransform` (`self.DefaultSceneRoot`))) (* (.scale (`SceneComponent.GetRelativeTransform` (`self.DefaultSceneRoot`))) (`BoxComponent.BoxExtent` (`self.Box`)))) (struct :`Pitch` 50.0) (`KismetMathLibrary.Conv_DoubleToVector` (* (`KismetMathLibrary.RandomFloatInRange` (`self.MinMeteorScale`) (`self.MaxMeteorScale`)) (`self.RagnarokDangerRatio`)))) "Undefined" "OverrideRootScale" null null))

(fn `StartRagnarok`
  (bind _fadeduration (`self.FadeDuration`))
  (`self.SetActorTickEnabled` true)
  (`AudioComponent.FadeOut` (`self.MusicSound`) _fadeduration 0.0 "Linear")
  (bind _returnvalue (`GameplayStatics.SpawnSound2D` "/Game/DinoGame/Audio/Music/Ragnarok_Cue.Ragnarok_Cue" 1.0 1.0 0.0 null))
  (`AudioComponent.FadeIn` _returnvalue _fadeduration 1.0 0.0 "Linear")
  (`KismetSystemLibrary.PrintString` "START RAGNAROK" true true (struct :`R` 1.0 :`G` 0.359522 :`A` 1.0)))

(fn `UserConstructionScript`)